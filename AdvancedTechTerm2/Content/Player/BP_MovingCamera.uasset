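; BP_MovingCamera is a player camera actor that other code repositions, either instantly or through an animated move.
; MoveCamera sets the actor location directly to the given position.
; TransitionCamera stores the current location, then plays the CameraTransition timeline to lerp toward the end location with teleporting moves.
; When the timeline finishes, it calls the CameraReachedDestination dispatcher to signal arrival.
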(event `MoveCamera`
  (params (Position :type "Vector Structure"))
  (`self.K2_SetActorLocation` self Position false false))

(event `TransitionCamera`
  (params (EndLocation :type "Vector Structure"))
  (set `self.StartLocation` (`self.K2_GetActorLocation`))
  (bind (_direction _transition) (`Timeline|CameraTransition` :!via `PlayFromStart`)
    (:`Update`
      (`self.K2_SetActorLocation` self (`KismetMathLibrary.VLerp` (`self.StartLocation`) EndLocation _transition) false true))
    (:`Finished`
      (`self.CameraReachedDestination`))))

(fn `UserConstructionScript`)