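; Player golf ball for a single-switch golf game, running a state machine of aim, hit, wait and end phases.
; One input, in Automatic or Inverse (hold-and-release) mode, stops a timer-rotated aim arrow, then a timeline power meter, to launch the physics ball by impulse.
; A polling timer detects rest and moves the drone camera, whose arrival callback starts the next phase.
; An undo countdown widget steps back, and respawns follow the checkpoint-frequency setting.
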(event `self.ReceiveBeginPlay`
  (bind _cameradrone (`self.CameraDrone`))
  (bind _papersprite (`self.PaperSprite`))
  (bind (_returnvalue_x _returnvalue_y) (`KismetMathLibrary.BreakVector` (`SceneComponent.K2_GetComponentLocation` (`self.GolfBallMesh`))))
  (`|ExecutionSequence`
    (:`then_0`
      (bind _asbp_settings (cast `/Game/Blueprints/BP_Settings` (`GameplayStatics.GetGameInstance`)))
      (bind _settings (`/Game/Blueprints/BP_Settings.GetSettings` _asbp_settings))
      (bind _output_get (set `self.Settings` _settings))
      (bind ((`SingleSwitchMethodGameplay_8_EFB662574D7237535507F99A5BB90F49` _singleswitchmethodgameplay) (`CheckpointFrequency_43_8B0D517E470F7F8CF0819AABE0C229BA` _checkpointfrequency)) (break `/Game/Blueprints/S_Settings` _output_get))
      (set `self.Single Switch Method Gameplay` _singleswitchmethodgameplay)
      (set `self.Checkpoint Frequency` _checkpointfrequency))
    (:`then_1`
      (bind _returnvalue (`GameplayStatics.GetActorOfClass` "/Game/Player/BP_MovingCamera.BP_MovingCamera_C"))
      (bind _output_get_2 (set `self.CameraDrone` _returnvalue))
      (`PlayerController.SetViewTargetWithBlend` (`GameplayStatics.GetPlayerController` 0) _output_get_2 0.0 "VTBlend_Linear" 0.0 false)
      (`/Game/Player/BP_MovingCamera.MoveCamera` _cameradrone (`KismetMathLibrary.MakeVector` _returnvalue_x _returnvalue_y (`self.Camera Distance`)))
      (add `/Game/Player/BP_MovingCamera.CameraReachedDestination` _cameradrone (delegate `Transition to AimPhase`)))
    (:`then_2`
      (bind _output_get_3 (set `self.CurrentState` "NewEnumerator0"))
      (`self.StateChange` _output_get_3)
      (bind _returnvalue_2 (`KismetSystemLibrary.K2_SetTimer` null "UpdateAngle" 0.01 true))
      (set `self.BallAimTimer` _returnvalue_2)
      (switch `/Game/Blueprints/Enums/E_SelectionState` (`self.Single Switch Method Gameplay`)
        (:`NewEnumerator0`
          _)
        (:`NewEnumerator1`
          (`KismetSystemLibrary.K2_PauseTimerHandle` (`self.BallAimTimer`))))
      (`SceneComponent.SetWorldScale3D` _papersprite (* (`SceneComponent.K2_GetComponentScale` _papersprite) (`.UIsize_36_B162DF55423A955841380C96AC7B64C4` (break `/Game/Blueprints/S_Settings` (`self.Settings`)))))
      (set `self.Number of Shots` 0)
      (bind _output_get_4 (set `self.StartPos` (`SceneComponent.K2_GetComponentLocation` (`self.GolfBallMesh`))))
      (bind _output_get_5 (set `self.LastPos` _output_get_4))
      (bind _output_get_6 (set `self.CurrentPos` _output_get_5))
      (set `self.CheckpointObjectPos` _output_get_6))
    (:`then_3`
      (bind _returnvalue_3 (`|CreateWidget` "/Game/UI/UsefulWidgets/WBP_UndoTimer.WBP_UndoTimer_C"))
      (bind _output_get_7 (set `self.UndoTimerUI` _returnvalue_3))
      (add `/Game/UI/UsefulWidgets/WBP_UndoTimer.TimerComplete` _output_get_7 (delegate `TimeFinished`))
      (`UserWidget.AddToViewport` _output_get_7 0))))

(event `TimeFinished`
  (bind (_lastpos_x _lastpos_y) (`KismetMathLibrary.BreakVector` (`self.LastPos`)))
  (switch `/Game/Blueprints/Enums/E_GameState` (`self.CurrentState`)
    (:`NewEnumerator0`
      (set `self.UndoHit` true)
      (`SceneComponent.K2_SetWorldLocation` (`self.GolfBallMesh`) (`self.LastPos`) false true)
      (`SceneComponent.SetVisibility` (`self.PaperSprite`) false false)
      (`/Game/Player/BP_MovingCamera.TransitionCamera` (`self.CameraDrone`) (`KismetMathLibrary.MakeVector` _lastpos_x _lastpos_y (`self.Camera Distance`)) false true))
    (:`NewEnumerator1`
      (`self.Transition to AimPhase` false))))

(event `self.ReceiveTick`
  (params (DeltaSeconds :type "Float (single-precision)"))
  (`self.K2_SetActorLocation` (`SceneComponent.K2_GetComponentLocation` (`self.GolfBallMesh`)) false true))

(event `Transition to AimPhase`
  (params (Repsawn :type Boolean) (Undo :type Boolean))
  (bind _directionfacing (`self.DirectionFacing`))
  (bind _undotimerui (`self.UndoTimerUI`))
  ;[0 0.1188 0.15 0.5] State Transitions and checks
  ;;[0.15 0.0545 0 0.5] Transition to the aim phase once the camera has caught up with the ball, if in the win area then transition to end state
  (if Undo
    (set `self.UndoHit` false)
    (`self.EnterFireState`)
    (switch `/Game/Blueprints/Enums/E_SelectionState` (`self.Single Switch Method Gameplay`)
      (:`NewEnumerator0`
        _)
      (:`NewEnumerator1`
        (`/Game/UI/UsefulWidgets/WBP_UndoTimer.EndTimer` (`self.UndoTimerUI`))
        (`self.StopPowerMeter`)))
    (`SceneComponent.SetVisibility` (`self.PaperSprite`) true false)
    (`SceneComponent.K2_SetWorldRotation` (`self.DirectionFacing`) (`self.PreviousRotation`) false false)
    (`self.K2_SetActorLocation` (`SceneComponent.K2_GetComponentLocation` (`self.GolfBallMesh`)) false true :!label _label)
    (else
      (set `self.CanHitBall` true)
      (if (`KismetArrayLibrary.Array_IsNotEmpty` (`PrimitiveComponent.GetOverlappingActors` (`self.GolfBallMesh`) "/Game/Blueprints/BP_Goal.BP_Goal_C"))
        (bind _output_get (set `self.CurrentState` "NewEnumerator2"))
        (`self.StateChange` _output_get (`self.Number of Shots`))
        (`SceneComponent.SetVisibility` (`self.PaperSprite`) false false)
        (else
          (bind _output_get_2 (set `self.CurrentState` "NewEnumerator0"))
          (`self.StateChange` _output_get_2)
          (`SceneComponent.SetVisibility` (`self.PaperSprite`) true false)
          (switch `/Game/Blueprints/Enums/E_SelectionState` (`self.Single Switch Method Gameplay`)
            (:`NewEnumerator0`
              (`KismetSystemLibrary.K2_UnPauseTimerHandle` (`self.BallAimTimer`)))
            (:`NewEnumerator1`
              _))
          (set `self.PreviousRotation` (`SceneComponent.K2_GetComponentRotation` _directionfacing))
          (`SceneComponent.K2_SetWorldRotation` :`self` _directionfacing)
          (if Repsawn
            _
            (else
              (`/Game/UI/UsefulWidgets/WBP_UndoTimer.StartTimer` _undotimerui)
              (goto _label)))))
      (`/Game/UI/UsefulWidgets/WBP_UndoTimer.EndTimer` _undotimerui))))

(event `UpdateAngle`
  (bind _directionfacing (`self.DirectionFacing`))
  (bind (_returnvalue_roll _returnvalue_pitch _returnvalue_yaw) (`KismetMathLibrary.BreakRotator` (`SceneComponent.K2_GetComponentRotation` _directionfacing)))
  ;[0.15 0.06382 0.09597 0.5] UI updates
  ;;[0.15 0.1285 0 0.5] Update Aim UI
  (`SceneComponent.K2_SetWorldRotation` _directionfacing (`KismetMathLibrary.MakeRotator` _returnvalue_roll _returnvalue_pitch (+ _returnvalue_yaw (* (`self.BaseArrowSpeed`) (`.UISpeed_35_9C4D7646416622D2614D00871F938AB9` (break `/Game/Blueprints/S_Settings` (`self.Settings`)))))) false true))

(event `UpdatePowerMeter`
  (bind ((`OverallAudio_24_B2994BAD44254C6C1A8E4BB3C9CEABE3` _overallaudio) (`EffectsAudio_27_C0A3745248A240CE6BE791929259B588` _effectsaudio)) (break `/Game/Blueprints/S_Settings` (`self.Settings`)))
  ;[0.15 0.06382 0.09597 0.5] UI updates
  ;;[0.15 0.1024 0 0.5] Update on screen power meter
  (`TimelineComponent.SetPlayRate` (`self.PowerUpdate`) (* (`.UISpeed_35_9C4D7646416622D2614D00871F938AB9` (break `/Game/Blueprints/S_Settings` (`self.Settings`))) (`self.BaseMeterSpeed`)))
  (`AudioComponent.Play` (`self.BarAudio`) 0.0)
  (bind (_direction _updatepower) (`Timeline|PowerUpdate` :!via `PlayFromStart`)
    (:`Update`
      (`|ExecutionSequence`
        (:`then_0`
          (set `self.ShotPower` (`KismetMathLibrary.Lerp` (`self.MinPower`) (`self.MaxPower`) _updatepower))
          (`self.PowerMeterUpdated` _updatepower))
        (:`then_1`
          (`AudioComponent.SetVolumeMultiplier` (`self.BarAudio`) (* _overallaudio _effectsaudio _updatepower 1.5)))))))

(event `CheckBallStopState`
  (bind (_returnvalue_x _returnvalue_y) (`KismetMathLibrary.BreakVector` (`SceneComponent.K2_GetComponentLocation` (`self.GolfBallMesh`))))
  ;[0 0.1188 0.15 0.5] State Transitions and checks
  ;;[0.15 0 0.0469 0.5] checks regularly if the ball has stopped, then transitions to the next phase
  (`self.CheckIfBallStopped`)
  (if (not (`self.IsBallMoving?`))
    (`KismetSystemLibrary.K2_ClearAndInvalidateTimerHandle` (`self.BallStopTimer`))
    (`/Game/Player/BP_MovingCamera.TransitionCamera` (`self.CameraDrone`) (`KismetMathLibrary.MakeVector` _returnvalue_x _returnvalue_y (`self.Camera Distance`)) false false)
    (set `self.CurrentPos` (`SceneComponent.K2_GetComponentLocation` (`self.GolfBallMesh`)))))

(event `StopPowerMeter`
  ;[0.15 0.06382 0.09597 0.5] UI updates
  ;;[0.15 0.1024 0 0.5] Update on screen power meter
  (`TimelineComponent.Stop` (`self.PowerUpdate`))
  (`AudioComponent.Stop` (`self.BarAudio`)))

(event `EnhancedInput|/Game/ThirdPerson/Input/Actions/IA_Automatic`
  (params (ActionValue :type Boolean) (ElapsedSeconds :type "Float (double-precision)") (TriggeredSeconds :type "Float (double-precision)") (InputAction :type "InputAction Object Reference" :default "/Game/ThirdPerson/Input/Actions/IA_Automatic.IA_Automatic"))
  ;[0 0.15 0.03326 0.5] Single input handling
  (:`Started`
    (switch `/Game/Blueprints/Enums/E_SelectionState` (`self.Single Switch Method Gameplay`)
      (:`NewEnumerator0`
        (switch `/Game/Blueprints/Enums/E_GameState` (`self.CurrentState`)
          (:`NewEnumerator0`
            (`self.EnterFireState`))
          (:`NewEnumerator1`
            (`/Game/UI/UsefulWidgets/WBP_UndoTimer.EndTimer` (`self.UndoTimerUI`))
            (`self.EnterWaitPhase`)))))))

(event `EnterFireState`
  ;[0 0.1188 0.15 0.5] State Transitions and checks
  ;;[0.1395 0 0.15 0.5] Transition the player to the fire phase
  (`/Game/UI/UsefulWidgets/WBP_UndoTimer.StartTimer` (`self.UndoTimerUI`))
  (`KismetSystemLibrary.K2_PauseTimerHandle` (`self.BallAimTimer`))
  (bind _output_get (set `self.CurrentState` "NewEnumerator1"))
  (`self.StateChange` _output_get)
  (`self.UpdatePowerMeter`))

(event `EnterWaitPhase`
  (bind _golfballmesh (`self.GolfBallMesh`))
  (bind ((`OverallAudio_24_B2994BAD44254C6C1A8E4BB3C9CEABE3` _overallaudio) (`EffectsAudio_27_C0A3745248A240CE6BE791929259B588` _effectsaudio)) (break `/Game/Blueprints/S_Settings` (`self.Settings`)))
  ;[0 0.1188 0.15 0.5] State Transitions and checks
  ;;[0 0.15 0.03236 0.5] Hit Phase
  (if (`self.CanHitBall`)
    (`self.StopPowerMeter`)
    (`SceneComponent.SetVisibility` (`self.PaperSprite`) false false)
    (set `self.LastPos` (`SceneComponent.K2_GetComponentLocation` _golfballmesh))
    (`PrimitiveComponent.AddImpulse` _golfballmesh (* (`SceneComponent.GetForwardVector` (`self.DirectionFacing`)) (`self.ShotPower`)) "None" false)
    (`GameplayStatics.PlaySound2D` (`KismetArrayLibrary.Array_Random` (`self.AudioSamplesHit`)) (* _overallaudio _effectsaudio) 1.0 0.0 null null)
    (set `self.CanHitBall` false)
    (set `self.IsBallMoving?` true)
    (bind _output_get (set `self.CurrentState` "NewEnumerator4"))
    (`self.StateChange` _output_get)
    (bind _returnvalue (`KismetSystemLibrary.K2_SetTimer` null "CheckBallStopState" 0.1 true))
    (set `self.BallStopTimer` _returnvalue)
    (`/Engine/EditorBlueprintResources/StandardMacros.IncrementInt` (`self.Number of Shots`))))

(event `EnhancedInput|/Game/ThirdPerson/Input/Actions/IA_Inverse`
  (params (ActionValue :type Boolean) (ElapsedSeconds :type "Float (double-precision)") (TriggeredSeconds :type "Float (double-precision)") (InputAction :type "InputAction Object Reference" :default "/Game/ThirdPerson/Input/Actions/IA_Inverse.IA_Inverse"))
  ;[0 0.15 0.03326 0.5] Single input handling
  (:`Started`
    (switch `/Game/Blueprints/Enums/E_SelectionState` (`self.Single Switch Method Gameplay`)
      (:`NewEnumerator1`
        (switch `/Game/Blueprints/Enums/E_GameState` (`self.CurrentState`)
          (:`NewEnumerator0`
            (`KismetSystemLibrary.K2_UnPauseTimerHandle` (`self.BallAimTimer`)))
          (:`NewEnumerator1`
            (`self.UpdatePowerMeter`))))))
  (:`Completed`
    (switch `/Game/Blueprints/Enums/E_SelectionState` (`self.Single Switch Method Gameplay`)
      (:`NewEnumerator1`
        (switch `/Game/Blueprints/Enums/E_GameState` (`self.CurrentState`)
          (:`NewEnumerator0`
            (`self.EnterFireState`)
            (`self.StopPowerMeter`))
          (:`NewEnumerator1`
            (`/Game/UI/UsefulWidgets/WBP_UndoTimer.EndTimer` (`self.UndoTimerUI`))
            (`self.EnterWaitPhase`)))))))

(event `Respawn`
  ;[1 0 0 0.261] Checkpoint Frequency Logic
  (`KismetSystemLibrary.K2_ClearAndInvalidateTimerHandle` (`self.BallStopTimer`))
  (`KismetSystemLibrary.Delay` 0.25)
  (`SceneComponent.SetHiddenInGame` (`self.GolfBallMesh`) true false)
  (`KismetSystemLibrary.Delay` 0.25)
  (switch `/Game/Blueprints/Enums/E_CheckpointFrequency` (`self.Checkpoint Frequency`)
    (:`NewEnumerator0`
      (`self.RespawnBasedOnEnum` (`self.StartPos`)))
    (:`NewEnumerator1`
      (`self.RespawnBasedOnEnum` (`self.CheckpointObjectPos`)))
    (:`NewEnumerator2`
      (`self.RespawnBasedOnEnum` (`self.CurrentPos`))))
  (`SceneComponent.SetHiddenInGame` (`self.GolfBallMesh`) false false))

(event `Set Checkpoint Object`
  (params (Location :type "Vector Structure"))
  ;[1 0 0 0.261] Checkpoint Frequency Logic
  (if (`|EnumEquality` (`self.Checkpoint Frequency`) "NewEnumerator1")
    (set `self.CheckpointObjectPos` Location)))

(fn `CheckIfBallStopped`
  (bind _golfballmesh (`self.GolfBallMesh`))
  (bind _returnvalue (`PrimitiveComponent.GetPhysicsLinearVelocity` (`self.GolfBallMesh`) "None"))
  (if (<= (`KismetMathLibrary.VSize` _returnvalue) 20.0)
    (`PrimitiveComponent.SetPhysicsLinearVelocity` _golfballmesh (0.0 0.0 0.0) false "None")
    (`PrimitiveComponent.SetPhysicsAngularVelocityInDegrees` _golfballmesh (0.0 0.0 0.0) false "None")
    (set `self.IsBallMoving?` false)
    (return)))

(fn `RespawnBasedOnEnum`
  (params (Pos :type "Vector Structure"))
  (bind _golfballmesh (`self.GolfBallMesh`))
  (bind (_returnvalue_x _returnvalue_y) (`KismetMathLibrary.BreakVector` (`SceneComponent.K2_GetComponentLocation` (`self.GolfBallMesh`))))
  (`SceneComponent.K2_SetWorldLocation` (`self.GolfBallMesh`) Pos false true)
  (`self.K2_SetActorLocation` Pos false true)
  (`/Game/Player/BP_MovingCamera.TransitionCamera` (`self.CameraDrone`) (`KismetMathLibrary.MakeVector` _returnvalue_x _returnvalue_y (`self.Camera Distance`)) true false)
  (`PrimitiveComponent.SetPhysicsLinearVelocity` _golfballmesh (0.0 0.0 0.0) false "None")
  (`PrimitiveComponent.SetPhysicsAngularVelocityInDegrees` _golfballmesh (0.0 0.0 0.0) false "None")
  (message `NavMovementInterface.StopActiveMovement` _golfballmesh))

(fn `UserConstructionScript`)