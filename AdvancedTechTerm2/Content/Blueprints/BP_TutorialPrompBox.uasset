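; BP_TutorialPrompBox is a trigger volume that shows a tutorial prompt while the golf ball is inside it.
; On BeginPlay it creates a Tutorial widget configured with its SetupString and optionally displays it immediately via ShowOnStart.
; Box overlap events, filtered to BP_GolfBall, add the widget to the viewport on entry and remove it on exit.
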(event `self.ReceiveBeginPlay`
  (bind _returnvalue (`|CreateWidget` (`self.Tutorial`) null (`self.SetupString`)))
  (set `self.TutorialUI` _returnvalue)
  (if (`self.ShowOnStart`)
    (`UserWidget.AddToViewport` (`self.TutorialUI`) 0)))

(event `self.Box.OnComponentBeginOverlap`
  (params (OverlappedComponent :type "PrimitiveComponent Object Reference") (OtherActor :type "Actor Object Reference") (OtherComp :type "PrimitiveComponent Object Reference") (OtherBodyIndex :type Integer) (bFromSweep :type Boolean) (SweepResult :type "HitResult Structure (by ref)"))
  (cast `/Game/Player/BP_GolfBall` OtherActor)
  (`UserWidget.AddToViewport` (`self.TutorialUI`) 0))

(event `self.Box.OnComponentEndOverlap`
  (params (OverlappedComponent :type "PrimitiveComponent Object Reference") (OtherActor :type "Actor Object Reference") (OtherComp :type "PrimitiveComponent Object Reference") (OtherBodyIndex :type Integer))
  (cast `/Game/Player/BP_GolfBall` OtherActor)
  (`Widget.RemoveFromParent` (`self.TutorialUI`)))

(fn `UserConstructionScript`)