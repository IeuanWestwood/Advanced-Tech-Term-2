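; BP_Settings manages persistent game settings stored in a BP_SaveData save game object.
; Init loads that object from the named save slot, or creates a fresh one if none exists.
; GetSettings returns the stored Settings, while SaveSettings overwrites them and immediately writes the save object back to the slot.
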(event `self.ReceiveInit`
  (bind _slot_name (`self.Slot Name`))
  (bind _returnvalue (`GameplayStatics.DoesSaveGameExist` _slot_name))
  (if _returnvalue
    (bind _returnvalue_2 (`GameplayStatics.LoadGameFromSlot` _slot_name))
    (bind _asbp_save_data (cast `/Game/Blueprints/BP_SaveData` _returnvalue_2))
    (set `self.SaveData` _asbp_save_data)
    (else
      (bind _returnvalue_3 (`GameplayStatics.CreateSaveGameObject` "/Game/Blueprints/BP_SaveData.BP_SaveData_C"))
      (set `self.SaveData` _returnvalue_3))))

(event `SaveGameData`
  (`GameplayStatics.SaveGameToSlot` (`self.SaveData`) (`self.Slot Name`)))

(fn `GetSettings`
  (returns (Settings :type "/Game/Blueprints/S_Settings Structure"))
  (return (`/Game/Blueprints/BP_SaveData.Settings` (`self.SaveData`))))

(fn `SaveSettings`
  (params (Settings :type "/Game/Blueprints/S_Settings Structure"))
  (set `/Game/Blueprints/BP_SaveData.Settings` Settings (`self.SaveData`))
  (`self.SaveGameData`)
  (return))